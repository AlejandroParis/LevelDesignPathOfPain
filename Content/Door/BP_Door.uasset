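; BP_Door is a double door that the player character can open.
; A sphere trigger sets the Door reference on MyCharacter when it enters and clears it when it leaves.
; The OpenDoor event instantly rotates the two leaves 90 degrees in opposite directions, with no animation, closing logic or guard against repeat calls.
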(event `OpenDoor`
  (`SceneComponent.K2_AddLocalRotation` (`self.door1`) (struct :`Yaw` 90.0) false false)
  (`SceneComponent.K2_AddLocalRotation` (`self.door2`) (struct :`Yaw` -90.0) false false))

(event `self.Sphere.OnComponentBeginOverlap`
  (params (OverlappedComponent :type "PrimitiveComponent Object Reference") (OtherActor :type "Actor Object Reference") (OtherComp :type "PrimitiveComponent Object Reference") (OtherBodyIndex :type Integer) (bFromSweep :type Boolean) (SweepResult :type "HitResult Structure (by ref)"))
  (bind _asmy_character (cast `/Game/Character/MyCharacter` OtherActor))
  (set `/Game/Character/MyCharacter.door` self _asmy_character))

(event `self.Sphere.OnComponentEndOverlap`
  (params (OverlappedComponent :type "PrimitiveComponent Object Reference") (OtherActor :type "Actor Object Reference") (OtherComp :type "PrimitiveComponent Object Reference") (OtherBodyIndex :type Integer))
  (bind _asmy_character (cast `/Game/Character/MyCharacter` OtherActor))
  (set `/Game/Character/MyCharacter.door` null _asmy_character))

(fn `UserConstructionScript`)